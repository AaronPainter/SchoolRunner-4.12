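; Interactive door actor that the player swings open and closed with the F key, named as a right-hand, 90-degree variant.
; A trigger box enables the actor's input on overlap and disables it when overlap ends, without filtering the overlapping actor.
; Each press flips DoorStatus and plays or reverses the DoorRotation timeline, whose track sets the whole actor's relative yaw.
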(event `self.TriggerBox.OnComponentBeginOverlap`
  (params (OverlappedComponent :type "PrimitiveComponent Object Reference") (OtherActor :type "Actor Object Reference") (OtherComp :type "PrimitiveComponent Object Reference") (OtherBodyIndex :type Integer) (bFromSweep :type Boolean) (SweepResult :type "HitResult Structure (by ref)"))
  (`self.EnableInput` (`GameplayStatics.GetPlayerController` 0)))

(event `Key|F`
  (params (Key :type "Key Structure" :default "AnyKey"))
  (:`Pressed`
    (if (`self.DoorStatus`)
      (set `self.DoorStatus` false)
      (bind (_direction _doorrot) (`Timeline|DoorRotation` :!label _label)
        (:`Update`
          (`self.K2_SetActorRelativeRotation` (`KismetMathLibrary.MakeRotator` 0.0 0.0 _doorrot))))
      (else
        (set `self.DoorStatus` true)
        (goto _label :!via `Reverse`)))))

(event `self.TriggerBox.OnComponentEndOverlap`
  (params (OverlappedComponent :type "PrimitiveComponent Object Reference") (OtherActor :type "Actor Object Reference") (OtherComp :type "PrimitiveComponent Object Reference") (OtherBodyIndex :type Integer))
  (`self.DisableInput` (`GameplayStatics.GetPlayerController` 0)))

(fn `UserConstructionScript`)